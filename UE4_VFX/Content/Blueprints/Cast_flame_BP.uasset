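; Flame cast effect Blueprint that sets up and animates the materials of its particle system.
; On BeginPlay it creates dynamic instances for two Dot_M elements and one Flamesprite_M element.
; The flame sprite material receives a one-time bone rotation from the first Testanim actor, packed into a color vector parameter.
; The cast event then plays a timeline that drives the "vis" scalar on both dot materials.
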(event Custom|cast
  (bind _newtrack_0 (Timeline|Timeline_0 Play)
    (:Update
      (Rendering|Material|SetScalarParameterValue (stale EventBeginPlay _returnvalue) "vis" _newtrack_0 :!class /Script/Engine.MaterialInstanceDynamic))))

(event EventBeginPlay
  (bind _particlesystem (Variables|Default|GetParticleSystem))
  (bind _returnvalue (Rendering|Material|CreateDynamicMaterialInstance _particlesystem 0 "/Game/Materials/Dot_M.Dot_M" :!class /Script/Engine.PrimitiveComponent))
  (bind _returnvalue_2 (Rendering|Material|CreateDynamicMaterialInstance _particlesystem 1 "/Game/Materials/Dot_M.Dot_M" :!class /Script/Engine.PrimitiveComponent))
  (bind _returnvalue_3 (Rendering|Material|CreateDynamicMaterialInstance _particlesystem 2 "/Game/Materials/flamesprite_M.flamesprite_M" :!class /Script/Engine.PrimitiveComponent))
  (bind _outactors (Actor|GetAllActorsOfClass "/Game/Blueprints/testanim.testanim_C"))
  (Rendering|Material|SetVectorParameterValue _returnvalue_3 "bonerotation" (Utilities|Struct|MakeLinearColor (.Roll (Math|Rotator|BreakRotator (.Rotation (Math|Transform|BreakTransform (Variables|/Game/Blueprints/testanim.testanim_C|Getbonetransform (Utilities|Array|Get(acopy) _outactors)))))) (.Pitch (Math|Rotator|BreakRotator (.Rotation (Math|Transform|BreakTransform (Variables|/Game/Blueprints/testanim.testanim_C|Getbonetransform (Utilities|Array|Get(acopy) _outactors)))))) (.Yaw (Math|Rotator|BreakRotator (.Rotation (Math|Transform|BreakTransform (Variables|/Game/Blueprints/testanim.testanim_C|Getbonetransform (Utilities|Array|Get(acopy) _outactors)))))) 0.0) :!class /Script/Engine.MaterialInstanceDynamic)
  (CallFunction|Cast))

(fn ConstructionScript)